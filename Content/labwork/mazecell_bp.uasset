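; Maze cell actor that builds one square tile of a maze, with a floor and optional walls on its four sides.
; The construction script derives wall length and thickness from the grid size, then scales the floor to match.
; Each enabled side flag adds a static mesh wall, scaled through a size-to-scale helper and offset to the far edge for north and east.
; The event graph holds no logic.
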(event EventBeginPlay)

(event Collision|EventActorBeginOverlap
  (params (OtherActor :type Actor%20Object%20Reference)))

(event EventTick
  (params (DeltaSeconds :type Float%20%28single-precision%29)))

(fn ConstructionScript
  (bind _grid_size (Variables|Default|Getgrid%20size))
  (LocalVariables|Setwalllenght _grid_size)
  (LocalVariables|Setwallthickness (* _grid_size 0.1))
  (Transformation|SetRelativeScale3D (Variables|Default|Getfloor) (Utilities|SizetoScale (Math|Vector|MakeVector (LocalVariables|Getwalllenght) (LocalVariables|Getwalllenght) (LocalVariables|Getwallthickness))))
  (if (Variables|Default|Getwestwall)
    (AddComponent|AddStaticMeshComponent false (Math|Transform|MakeTransform "0, 0, 0" "0, 0, 0" (Utilities|SizetoScale (Math|Vector|MakeVector (LocalVariables|Getwalllenght) (LocalVariables|Getwallthickness) (LocalVariables|Getwallheight))))))
  (if (Variables|Default|Getsouthwall)
    (AddComponent|AddStaticMeshComponent false (Math|Transform|MakeTransform "0, 0, 0" "0, 0, 0" (Utilities|SizetoScale (Math|Vector|MakeVector (LocalVariables|Getwallthickness) (LocalVariables|Getwalllenght) (LocalVariables|Getwallheight))))))
  (if (Variables|Default|Getnorthwall)
    (AddComponent|AddStaticMeshComponent false (Math|Transform|MakeTransform (Math|Vector|MakeVector (- (LocalVariables|Getwalllenght) (LocalVariables|Getwallthickness)) 0.0 0.0) "0, 0, 0" (Utilities|SizetoScale (Math|Vector|MakeVector (LocalVariables|Getwallthickness) (LocalVariables|Getwalllenght) (LocalVariables|Getwallheight))))))
  (if (Variables|Default|Geteastwall)
    (AddComponent|AddStaticMeshComponent false (Math|Transform|MakeTransform (Math|Vector|MakeVector 0.0 (- (LocalVariables|Getwalllenght) (LocalVariables|Getwallthickness)) 0.0) "0, 0, 0" (Utilities|SizetoScale (Math|Vector|MakeVector (LocalVariables|Getwalllenght) (LocalVariables|Getwallthickness) (LocalVariables|Getwallheight)))))))