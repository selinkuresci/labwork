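; Swinging axe pendulum hazard that knocks back and damages the player.
; A timeline lerps the Axe's relative rotation between two opposite angles, switching between play and reverse each time it finishes to swing endlessly.
; A Box hit launches BP_ThirdPersonCharacter along the actor-to-box direction with a slight upward boost.
; Separately, actor overlap applies damage to anything tagged Player.
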(event OnComponentHit(Box)
  (params (HitComponent :type Primitive%20Component%20Object%20Reference) (OtherActor :type Actor%20Object%20Reference) (OtherComp :type Primitive%20Component%20Object%20Reference) (NormalImpulse :type Vector :default "0, 0, 0") (Hit :type Hit%20Result%20Structure%20%28by%20ref%29))
  (bind _asbp_third_person_character (Utilities|Casting|CastToBP_ThirdPersonCharacter OtherActor))
  (Character|LaunchCharacter _asbp_third_person_character (+ (* (Math|Vector|Normalize (- (Transformation|GetWorldLocation (Variables|Default|GetBox)) (Transformation|GetActorLocation))) 3e+03) (* (Transformation|GetActorUpVector) 1.5e+02)) false false))

(event Collision|EventActorBeginOverlap
  (params (OtherActor :type Actor%20Object%20Reference))
  (if (Actor|ActorHasTag OtherActor "Player")
    (Game|Damage|ApplyDamage OtherActor 1e+01 0 0)))

(event EventBeginPlay
  (bind (_direction _movement) (Timeline|Timeline Play)
    (:Update
      (Transformation|SetRelativeRotation (Variables|Default|Getaxe) (Math|Rotator|Lerp(Rotator) "0.000000,0.000000,-20.000000" "0.000000,0.000000,20.000000" _movement) false false))
    (:Finished
      (if (Utilities|Enum|Equal(Enum) "Forward" _direction)
        (Timeline|Timeline Reverse)
        (else
          (Timeline|Timeline Play))))))

(fn ConstructionScript)